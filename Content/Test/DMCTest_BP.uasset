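; DMCTest_BP is a test Blueprint for a DeformMesh object that works with a procedural mesh and a static mesh.
; The construction script assigns ProceduralMesh and StaticMesh to DeformMesh, then calls Rebuild with false.
; BeginPlay calls Rebuild again with true, so the mesh is rebuilt both on construction and at game start.
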(event EventBeginPlay
  (Class|DeformMeshComponent|Rebuild (Variables|Default|GetDeformMesh) true))

(fn ConstructionScript
  (Variables|/Script/mesh_deformer.DeformMeshComponent|SetProceduralMeshComponent (Variables|Default|GetDeformMesh) (Variables|Default|GetProceduralMesh))
  (Variables|/Script/mesh_deformer.DeformMeshComponent|SetStaticMesh (Variables|Default|GetDeformMesh) (Variables|Default|GetStaticMesh))
  (Class|DeformMeshComponent|Rebuild (Variables|Default|GetDeformMesh) false))